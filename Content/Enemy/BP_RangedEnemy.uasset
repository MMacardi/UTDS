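; Ranged enemy Blueprint that supplies a rifle attack animation and passes its enemy index to the AI.
; Attack plays the hip-fire montage, prints a debug string, and broadcasts OnAttackEnd whether the montage completes or is interrupted.
; BeginPlay calls EnemyIndexAppearance, then after a short delay writes EnemyIndex to the AI controller's blackboard.
; No projectile or damage logic appears in these graphs.
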(event EventBeginPlay
  (CallFunction|EnemyIndexAppearance)
  (Utilities|FlowControl|Delay 0.2)
  (Class|BlackboardComponent|SetValueasInt (AI|GetBlackboard (AI|GetAIController self)) (Variables|Default|GetEnemyIndexKeyName) (Variables|Default|GetEnemyIndex)))

(event EventAttack
  (Utilities|FlowControl|Sequence
    (:then_0
      (Animation|Montage|PlayMontage (Variables|Character|GetMesh) "/Game/EnemyRangedAnimation/Fire_Rifle_Hip_Montage.Fire_Rifle_Hip_Montage"
        (:OnCompleted
          _)
        (:OnInterrupted
          _))
      (Default|CallOnAttackEnd))
    (:then_1
      (Development|PrintString "attacked"))))

(fn ConstructionScript
  (|CallParentFunction))